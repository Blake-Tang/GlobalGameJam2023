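; Magic book actor that animates page flips with a Niagara effect and swaps the page textures shown on the book.
; Each flip activates the Pages effect, waits briefly, then advances the page counter to update the Book material's TextureChoice and the effect's AtlasChoice.
; BeginPlay runs one flip through ChangePage, while FlipBook adds a wrap-around of the counter and has no caller here, as the looping timer is unconnected.
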(event Custom|ChangePage
  (bind _pages (Variables|Default|GetPages))
  (Class|NiagaraComponent|SetVariableInt _pages "AtlasChoice" (+ (Variables|Default|GetNumPage) 1))
  (Components|Activation|Activate _pages true)
  (Utilities|FlowControl|Delay 0.25)
  (bind _result (Math|Integer|IncrementInt (Variables|Default|GetNumPage))
    (:%20%20
      (bind _output_get (Variables|Default|SetNumPage (- (* _result 2) 1)))
      (Rendering|Material|SetScalarParameterValueonMaterials (Variables|Default|GetBook) "TextureChoice" (Math|Conversions|ToFloat(Integer) _output_get))
      (Class|NiagaraComponent|SetVariableInt _pages "AtlasChoice" _output_get)
      (Variables|Default|SetNumPage _result))))

(event EventBeginPlay
  (CallFunction|ChangePage))

(event Collision|EventActorBeginOverlap
  (params (OtherActor :type Actor%20Object%20Reference)))

(event EventTick
  (params (DeltaSeconds :type Float%20%28single-precision%29)))

(event EventFlipBook
  (bind _pages (Variables|Default|GetPages))
  (if (>= (Variables|Default|GetNumPage) 5)
    (Variables|Default|SetNumPage 0))
  (Class|NiagaraComponent|SetVariableInt _pages "AtlasChoice" (+ (Variables|Default|GetNumPage) 1))
  (Components|Activation|Activate _pages true)
  (Utilities|FlowControl|Delay 0.25)
  (bind _result (Math|Integer|IncrementInt (Variables|Default|GetNumPage))
    (:%20%20
      (bind _output_get (Variables|Default|SetNumPage (- (* _result 2) 1)))
      (Rendering|Material|SetScalarParameterValueonMaterials (Variables|Default|GetBook) "TextureChoice" (Math|Conversions|ToFloat(Integer) _output_get))
      (Class|NiagaraComponent|SetVariableInt _pages "AtlasChoice" _output_get)
      (Variables|Default|SetNumPage _result))))

(fn ConstructionScript)