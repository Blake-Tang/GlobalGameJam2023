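; BP_BowlSystem is a potion-making bowl for one root ingredient type, with the construction script showing the matching plant bowl mesh.
; AddMeshToBowl spawns that type's ingredient mesh at a randomized offset and rotation around DropPoint and tracks it in Ref.
; BowlSelected removes one matching item from the player's CollectedItems, reports it to BP_PotionSystem, and destroys one tracked mesh, using DoOnce gates to limit each loop to a single item.
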(event Custom|AddMeshToBowl
  (bind _returnvalue (Math|Random|RandomFloatinRange 8.0 -8.0))
  (bind _returnvalue_2 (Math|Vector|MakeVector 1.0 1.0 1.0))
  (bind _drop_point (Variables|Default|GetDrop%20Point))
  (bind _returnvalue_3 (Transformation|GetWorldLocation _drop_point))
  (bind _returnvalue_4 (AddComponent|AddStaticMeshComponent false (Math|Transform|MakeTransform (Math|Vector|MakeVector (+ (.x _returnvalue_3) _returnvalue) (+ (.y _returnvalue_3) _returnvalue) (+ (.z _returnvalue_3) (Math|Random|RandomFloatinRange 0.0 17.0))) (Math|Random|RandomRotator false) (Utilities|Select :Index (Variables|Default|GetRootBowlType) :NewEnumerator0 "0.200000,0.200000,0.200000" :NewEnumerator1 _returnvalue_2 :NewEnumerator2 _returnvalue_2 :NewEnumerator3 _returnvalue_2))))
  (Components|StaticMesh|SetStaticMesh _returnvalue_4 (Utilities|Select :Index (Variables|Default|GetRootBowlType) :NewEnumerator0 "/Game/Art/Meshes/SM_EnemyDrop_Twigs.SM_EnemyDrop_Twigs" :NewEnumerator1 "/Game/Art/Meshes/SM_RootVegetable_Bud.SM_RootVegetable_Bud" :NewEnumerator2 "/Game/Art/Meshes/SM_SupportFoxGlove_Bud.SM_SupportFoxGlove_Bud" :NewEnumerator3 "/Game/Art/Meshes/SM_ThistleBud.SM_ThistleBud"))
  (Utilities|Array|Add (Variables|Default|GetRef) _returnvalue_4))

(event EventBowlSelected
  (bind _ref (Variables|Default|GetRef))
  (for (_array_element _array_index) (Variables|/Game/BP/Character/BP_BaseCharacter.BP_BaseCharacter_C|GetCollectedItems (Variables|Default|GetCharacter))
    (if (Utilities|Enum|Equal(Enum) _array_element (Variables|Default|GetRootBowlType))
      (Utilities|FlowControl|DoOnce false
        (:Completed
          (Class|BPICauldron|AddItem(Message) (Variables|Default|GetPotionSystem) (Variables|Default|GetRootBowlType))
          (Utilities|Array|RemoveIndex (Variables|/Game/BP/Character/BP_BaseCharacter.BP_BaseCharacter_C|GetCollectedItems (Variables|Default|GetCharacter)) _array_index)))))
  (for (_array_element_2 _array_index_2) _ref
    (Utilities|FlowControl|DoOnce false
      (:Completed
        (Components|DestroyComponent _array_element_2)
        (Utilities|Array|RemoveIndex _ref _array_index_2))))
  (Utilities|FlowControl|Sequence
    (:then_0
      (Utilities|FlowControl|DoOnce false) ; enters at Reset
    )
    (:then_1
      (Utilities|FlowControl|DoOnce false) ; enters at Reset
    )))

(event EventBeginPlay
  (bind _returnvalue (Actor|GetActorOfClass "/Game/BP/PotionMaking/BP_PotionSystem.BP_PotionSystem_C"))
  (Variables|Default|SetPotionSystem _returnvalue)
  (bind _asbp_base_character (Utilities|Casting|CastToBP_BaseCharacter (Game|Player|GetPlayerPawn 0)))
  (Variables|Default|SetCharacter _asbp_base_character))

(event EventTick
  (params (DeltaSeconds :type Float%20%28single-precision%29)))

(fn ConstructionScript
  (Development|SetHiddeninGame (Variables|Default|GetPlantBowlOne) (Utilities|Select :Index (Variables|Default|GetRootBowlType) :NewEnumerator0 false :NewEnumerator1 true :NewEnumerator2 true :NewEnumerator3 true) true)
  (Development|SetHiddeninGame (Variables|Default|GetPlantBowlTwo) (Utilities|Select :Index (Variables|Default|GetRootBowlType) :NewEnumerator0 true :NewEnumerator1 false :NewEnumerator2 true :NewEnumerator3 true) true)
  (Development|SetHiddeninGame (Variables|Default|GetPlantBowlThree) (Utilities|Select :Index (Variables|Default|GetRootBowlType) :NewEnumerator0 true :NewEnumerator1 true :NewEnumerator2 false :NewEnumerator3 true) true)
  (Development|SetHiddeninGame (Variables|Default|GetPlantBowlFour) (Utilities|Select :Index (Variables|Default|GetRootBowlType) :NewEnumerator0 true :NewEnumerator1 true :NewEnumerator2 true :NewEnumerator3 false) true))