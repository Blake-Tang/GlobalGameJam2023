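; BP_PotionSystem is a potion-crafting Blueprint that turns combinations of four root types into potions for the player.
; AddItem records each root, fires a starburst and sets per-type flags, so order and duplicates are ignored.
; Confirm runs FindPotion, whose sequenced branches let later matches override earlier ones.
; It then prints and sends the result to the player's inventory, even without a match, plays success or smoke VFX, and resets.
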(event Custom|ResetSystem
  (Utilities|Array|Clear (Variables|Default|GetRootsInSystem))
  (Utilities|SetAllFalse)
  (Utilities|SetNoPotion))

(event EventConfirm
  (bind _potiontype (Variables|Default|GetPotionType))
  (CallFunction|FindPotion)
  (Development|PrintString (Utilities|String|EnumtoString _potiontype))
  (Class|BPIItemObjects|AddtoInventory(Message) (Variables|Default|GetPlayer) _potiontype)
  (if (Utilities|Enum|NotEqual(Enum) _potiontype "NewEnumerator5")
    (Components|Activation|Activate (Variables|Default|GetVFX_StarBurst_2) true)
    (else
      (Components|Activation|Activate (Variables|Default|GetVFX_EXPSmoke) true)))
  (CallFunction|ResetSystem))

(event EventAddItem
  (params (Root :type E_Roots%20Enum :default "NewEnumerator0"))
  (bind _rootsinsystem (Variables|Default|GetRootsInSystem))
  (Components|Activation|Activate (Variables|Default|GetVFX_StarBurst) true)
  (Utilities|Array|Add _rootsinsystem Root)
  (for _array_element _rootsinsystem
    (switch Utilities|FlowControl|Switch|SwitchonE_Roots _array_element
      (:NewEnumerator0
        (Variables|Default|SetOne true))
      (:NewEnumerator1
        (Variables|Default|SetTwo true))
      (:NewEnumerator2
        (Variables|Default|SetThree true))
      (:NewEnumerator3
        (Variables|Default|SetFour true)))))

(event EventBeginPlay
  (CallFunction|ResetSystem)
  (bind _asbp_base_character (Utilities|Casting|CastToBP_BaseCharacter (Game|Player|GetPlayerPawn 0)))
  (Variables|Default|SetPlayer _asbp_base_character))

(fn ConstructionScript)

(fn FindPotion
  (Utilities|FlowControl|Sequence
    (:then_0
      (if (Variables|Default|GetOne)
        (if (Variables|Default|GetTwo)
          (Variables|Default|SetPotionType "NewEnumerator2")
          (elif (Variables|Default|GetFour)
            (if (Variables|Default|GetThree)
              (Variables|Default|SetPotionType "NewEnumerator4"))))))
    (:then_1
      (if (Variables|Default|GetTwo)
        (if (Variables|Default|GetThree)
          (Variables|Default|SetPotionType "NewEnumerator3")
          (elif (Variables|Default|GetFour)
            (Variables|Default|SetPotionType "NewEnumerator1")))))
    (:then_2
      (if (not (Variables|Default|GetOne))
        (if (Variables|Default|GetFour)
          (if (Variables|Default|GetThree)
            (Variables|Default|SetPotionType "NewEnumerator0")))))))