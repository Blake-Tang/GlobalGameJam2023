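; BP_Potion is a potion actor that applies an effect chosen by PotionType when its collision overlaps something, then spawns a type-specific burst and destroys itself.
; The construction script picks the matching potion mesh and stores its bounds.
; Boost, upgrade and heal types message the overlapped actor through interfaces, mainly BPI_Turret.
; Explosion deals massive damage via a sphere trace, while Bramble slows every BP_Enem in the level.
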(event OnComponentBeginOverlap(Collision)
  (params (OverlappedComponent :type Primitive%20Component%20Object%20Reference) (OtherActor :type Actor%20Object%20Reference) (OtherComp :type Primitive%20Component%20Object%20Reference) (OtherBodyIndex :type Integer) (bFromSweep :type Boolean) (SweepResult :type Hit%20Result%20Structure%20%28by%20ref%29))
  (bind _returnvalue (Utilities|DoesObjectImplementInterface OtherActor "/Game/BP/TurretPlants/BPI_Turret.BPI_Turret_C"))
  (bind _defaultsceneroot (Variables|Default|GetDefaultSceneRoot))
  (bind _returnvalue_2 (Transformation|GetWorldLocation _defaultsceneroot))
  (Utilities|FlowControl|Sequence
    (:then_0
      (Development|PrintString (Utilities|GetDisplayName OtherActor)))
    (:then_1
      (switch Utilities|FlowControl|Switch|SwitchonE_PotionType (Variables|Default|GetPotion%20Type)
        (:NewEnumerator0
          (if (Utilities|DoesObjectImplementInterface OtherActor "/Game/BP/TurretPlants/BPI_Turret.BPI_Turret_C")
            (Class|BPITurret|Boost(Message) OtherActor)
            (elif (Utilities|DoesObjectImplementInterface OtherActor "/Game/BP/BPI/BPI_ItemObjects.BPI_ItemObjects_C")
              (Class|BPIItemObjects|BoostItem(Message) OtherActor))))
        (:NewEnumerator1
          ;[1 1 1] Explosion
          (bind _outhits (Collision|MultiSphereTraceByChannel _returnvalue_2 _returnvalue_2 6e+02 "TraceTypeQuery1" false 0 "None"))
          (for _array_element _outhits
            (Utilities|IsValid (.HitActor (Collision|BreakHitResult _array_element))
              (:Is%20Valid
                (Class|BPIEnemy|DealDamage(Message) (.HitActor (Collision|BreakHitResult _array_element)) 1e+08)))))
        (:NewEnumerator2
          (if _returnvalue
            (Class|BPITurret|Upgrade(Message) OtherActor)))
        (:NewEnumerator3
          (if _returnvalue
            (Class|BPITurret|Heal(Message) OtherActor)))
        (:NewEnumerator4
          (bind _outactors (Actor|GetAllActorsOfClass "/Game/BP/Enemy/BP_Enem.BP_Enem_C"))
          (for _array_element_2 _outactors
            (Class|BPIEnemy|BrambleSlow(Message) _array_element_2)))))
    (:then_2
      (CallFunction|Explode))))

(event Custom|Explode
  (bind _cube (Variables|Default|GetCube))
  (Niagara|SpawnSystematLocation (Utilities|Select :Index (Variables|Default|GetPotion%20Type) :NewEnumerator0 "/Game/Stylized_VFX_StPack/Particles/UPDATE_1_3/P_IceExplosion.P_IceExplosion" :NewEnumerator1 "/Game/Stylized_VFX_StPack/Particles/UPDATE_1_4/P_Shockwave_Expl_03.P_Shockwave_Expl_03" :NewEnumerator2 "/Game/Stylized_VFX_StPack/Particles/UPDATE_1_3/P_IceExplosion.P_IceExplosion" :NewEnumerator3 "/Game/Stylized_VFX_StPack/Particles/UPDATE_1_3/P_IceExplosion.P_IceExplosion" :NewEnumerator4 "/Game/Stylized_VFX_StPack/Particles/UPDATE_1_3/P_IceExplosion.P_IceExplosion" :NewEnumerator5 0) (Transformation|GetActorLocation))
  (Utilities|IsValid _cube
    (:Is%20Valid
      _)
    (:Is%20Not%20Valid
      _))
  (Components|DestroyComponent _cube)
  (Actor|DestroyActor))

(event EventBeginPlay)

(event Collision|EventActorBeginOverlap
  (params (OtherActor :type Actor%20Object%20Reference)))

(event EventTick
  (params (DeltaSeconds :type Float%20%28single-precision%29)))

(fn ConstructionScript
  (bind _cube (Variables|Default|GetCube))
  (bind (_min _max) (Components|StaticMesh|GetLocalBounds _cube))
  (bind _returnvalue (- _max _min))
  (switch Utilities|FlowControl|Switch|SwitchonE_PotionType (Variables|Default|GetPotion%20Type)
    (:NewEnumerator0
      (Variables|Default|SetMesh "/Game/Art/Meshes/SM_Potion_1.SM_Potion_1"))
    (:NewEnumerator1
      (Variables|Default|SetMesh "/Game/Art/Meshes/SM_Potion_2.SM_Potion_2"))
    (:NewEnumerator2
      (Variables|Default|SetMesh "/Game/Art/Meshes/SM_Potion_3.SM_Potion_3"))
    (:NewEnumerator3
      (Variables|Default|SetMesh "/Game/Art/Meshes/SM_Potion_4.SM_Potion_4"))
    (:NewEnumerator4
      (Variables|Default|SetMesh "/Game/Art/Meshes/SM_Potion_5.SM_Potion_5")))
  (Components|StaticMesh|SetStaticMesh (Variables|Default|GetCube) (Variables|Default|GetMesh))
  (Variables|Default|SetcollisionSize _returnvalue)
  (Variables|Default|SetCollision%20Location%20Set (/ _returnvalue 2)))