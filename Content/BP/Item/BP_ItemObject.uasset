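; BP_ItemObject is a harvestable item with four RootType variants, its construction script showing only the matching mesh.
; Pickup adds a mesh to the BowlSystem (found only for type One), disables collision and timeline-lerps the selected component to the player before hiding and resetting it.
; A looping timer then restores visibility and collision after a random delay, shortened while BoostItem's temporary retriggerable boost is active.
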(event Custom|GrowBack
  (Development|SetHiddeninGame (Utilities|Select :Index (Variables|Default|GetRootType) :NewEnumerator0 (Variables|Default|GetOne) :NewEnumerator1 (Variables|Default|GetBudTwo) :NewEnumerator2 (Variables|Default|GetBudThree) :NewEnumerator3 (Variables|Default|GetBudFour)) false true)
  (Collision|SetActorEnableCollision true))

(event EventBoostItem
  (Development|PrintString "Boosted")
  (Variables|Default|SetBoosted true)
  (Utilities|FlowControl|RetriggerableDelay 15.0)
  (Variables|Default|SetBoosted false))

(event EventPickUpObject
  (bind _one (Variables|Default|GetOne))
  (bind _budthree (Variables|Default|GetBudThree))
  (bind _budfour (Variables|Default|GetBudFour))
  (bind _roottype (Variables|Default|GetRootType))
  (bind _budtwo (Variables|Default|GetBudTwo))
  (bind _one_2 (Variables|Default|GetOne))
  (bind _budthree_2 (Variables|Default|GetBudThree))
  (bind _budfour_2 (Variables|Default|GetBudFour))
  (bind _roottype_2 (Variables|Default|GetRootType))
  (bind _budtwo_2 (Variables|Default|GetBudTwo))
  (bind _returnvalue (Utilities|Select :Index _roottype :NewEnumerator0 _one_2 :NewEnumerator1 _budtwo :NewEnumerator2 _budthree_2 :NewEnumerator3 _budfour_2))
  (bind _returnvalue_2 (Utilities|Select :Index _roottype_2 :NewEnumerator0 _one :NewEnumerator1 _budtwo_2 :NewEnumerator2 _budthree :NewEnumerator3 _budfour))
  (bind _returnvalue_3 (Transformation|GetWorldLocation _returnvalue_2))
  (Default|AddMeshtoBowl (Variables|Default|GetBowlSystem))
  (Collision|SetActorEnableCollision false)
  (Variables|Default|SetGoBackToLocation _returnvalue_3)
  (bind _newtrack_0 (Timeline|Fly%20to%20Player PlayFromStart)
    (:Update
      (Transformation|SetWorldLocation _returnvalue_2 (Math|Vector|Lerp(Vector) _returnvalue_3 (Transformation|GetWorldLocation (Variables|/Game/BP/Character/BP_BaseCharacter.BP_BaseCharacter_C|GetLeft%20Click%20Start%20Location (Variables|Default|GetAs%20BP%20Base%20Character))) _newtrack_0) false false))
    (:Finished
      (Development|SetHiddeninGame _returnvalue true true)
      (Transformation|SetWorldLocation _returnvalue (Variables|Default|GetGoBackToLocation) false false)
      (Utilities|Time|SetTimerbyEvent (delegate Custom|GrowBack) (Math|Float|SelectFloat 1.0 (Math|Random|RandomFloatinRange 5.0 1e+01) (Variables|Default|GetBoosted)) true))))

(event EventUseObject)

(event EventBeginPlay
  (Utilities|FlowControl|Sequence
    (:then_0
      (bind _outactors (Actor|GetAllActorsOfClass "/Game/BP/PotionMaking/BP_BowlSystem.BP_BowlSystem_C"))
      (for _array_element _outactors
        (if (and (Utilities|Enum|Equal(Enum) (Variables|/Game/BP/PotionMaking/BP_BowlSystem.BP_BowlSystem_C|GetRootBowlType _array_element) "NewEnumerator0") (Utilities|Enum|Equal(Enum) (Variables|Default|GetRootType) "NewEnumerator0"))
          (Variables|Default|SetBowlSystem _array_element))))
    (:then_1
      (bind _asbp_base_character (Utilities|Casting|CastToBP_BaseCharacter (Game|Player|GetPlayerPawn 0)))
      (Variables|Default|SetAs%20BP%20Base%20Character _asbp_base_character))))

(fn ConstructionScript
  (Development|SetHiddeninGame (Variables|Default|GetOne) (Utilities|Select :Index (Variables|Default|GetRootType) :NewEnumerator0 false :NewEnumerator1 true :NewEnumerator2 true :NewEnumerator3 true) true)
  (Development|SetHiddeninGame (Variables|Default|GetTwo) (Utilities|Select :Index (Variables|Default|GetRootType) :NewEnumerator0 true :NewEnumerator1 false :NewEnumerator2 true :NewEnumerator3 true) true)
  (Development|SetHiddeninGame (Variables|Default|GetThree) (Utilities|Select :Index (Variables|Default|GetRootType) :NewEnumerator0 true :NewEnumerator1 true :NewEnumerator2 false :NewEnumerator3 true) true)
  (Development|SetHiddeninGame (Variables|Default|GetFour) (Utilities|Select :Index (Variables|Default|GetRootType) :NewEnumerator0 true :NewEnumerator1 true :NewEnumerator2 true :NewEnumerator3 false) true))