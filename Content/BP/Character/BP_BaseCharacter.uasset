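; Player character for a witch potion game, viewing the world through fixed, tag-assigned BP_CamSetting cameras.
; After an optional intro blend, WASD blends between views and shows only the active camera's hands.
; Left click uses interface checks on the cursor hit to collect items or use cauldron and bowl, otherwise spawns the selected potion from inventory.
; It also tracks house health for shake strength and losing, and manages menu widgets.
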(event Custom|Select%20Current%20Object
  (params (Potion%20Type :type E_PotionType%20Enum%20%28by%20ref%29 :default "NewEnumerator0"))
  ;[1 1 1] Select Current Object
  (Development|PrintString (Utilities|String|EnumtoString Potion%20Type))
  (Variables|Default|SetPotion%20Type Potion%20Type))

(event Custom|Reset%20Do%20Once%20Tab
  (bind _tab_menu (Variables|Widget|GetTab%20Menu))
  ;[1 1 1] Tab
  (Utilities|FlowControl|DoOnce false) ; enters at Reset
)

(event Custom|Play%20Cam%20Shake
  (bind _house_health (Variables|Default|GetHouse%20Health))
  ;[1 1 1] Cam Shake
  (if (> _house_health 75.0)
    (Variables|Default|SetShake "/Game/BP/CamShake/CustomCamShake_light.CustomCamShake_light_C")
    (elif (> _house_health 3e+01)
      (Variables|Default|SetShake "/Game/BP/CamShake/CustomCamShake_Medium.CustomCamShake_Medium_C")
      (else
        (Variables|Default|SetShake "/Game/BP/CamShake/CustomCamShake_Heavy.CustomCamShake_Heavy_C"))))
  (Camera|PlayWorldCameraShake (Variables|Default|GetShake) (Transformation|GetWorldLocation (Variables|Default|GetDefaultSceneRoot)) 5e+02 1e+03 1.0 true))

(event Custom|Damage%20House
  ;[1 1 1] Damage House
  (Variables|Default|SetHouse%20Health (- (Variables|Default|GetHouse%20Health) 2.0))
  (if (<= (Variables|Default|GetHouse%20Health) 0.0)
    (CallFunction|LoseGame)))

(event Custom|Lose%20Game
  ;[1 1 1] Lose Game
  (bind _returnvalue (UserInterface|CreateWidget "/Game/BP/Widget/Widget_Lose.Widget_Lose_C"))
  (bind _output_get (Variables|Default|Setlose%20widget _returnvalue))
  (UserInterface|Viewport|AddtoViewport _output_get 0))

(event Custom|First%20Blend
  (Game|Player|SetViewTargetwithBlend (Game|GetPlayerController 0) (Variables|Cam|GetForward%20Cam) 2.0 "VTBlend_Cubic" 0.0 true))

(event EventAddtoInventory
  (params (Potion :type E_PotionType%20Enum :default "NewEnumerator0"))
  (bind _inventory (Variables|Default|GetInventory))
  ;[1 1 1] Add To Inventory
  (Default|PlayHandAnimation (Variables|Cam|GetCurrentCam) (Utilities|Select :Index Potion :NewEnumerator0 "/Game/Art/Animations/Witch_PotionSuccess_02_Montage.Witch_PotionSuccess_02_Montage" :NewEnumerator1 "/Game/Art/Animations/Witch_PotionSuccess_02_Montage.Witch_PotionSuccess_02_Montage" :NewEnumerator2 "/Game/Art/Animations/Witch_PotionSuccess_02_Montage.Witch_PotionSuccess_02_Montage" :NewEnumerator3 "/Game/Art/Animations/Witch_PotionSuccess_02_Montage.Witch_PotionSuccess_02_Montage" :NewEnumerator4 "/Game/Art/Animations/Witch_PotionSuccess_02_Montage.Witch_PotionSuccess_02_Montage" :NewEnumerator5 "/Game/Art/Animations/Witch_PotionFail1_Montage.Witch_PotionFail1_Montage"))
  (bind _result (Math|Integer|IncrementInt (.Value (Utilities|Map|Find _inventory Potion)))
    (:%20%20
      (Utilities|Map|Add _inventory Potion _result)
      (for _index (range 0 5)
        _))))

(event EventBeginPlay
  ;[1 1 1] Begin Play
  (Variables|Cam|SetCam%20movement%20Locked true)
  (Utilities|FlowControl|Sequence
    (:then_0
      (bind _outactors (Actor|GetAllActorsOfClass "/Game/BP/Character/BP_CamSetting.BP_CamSetting_C"))
      (for _array_element _outactors
        (Variables|Cam|SetCurrent%20Instance _array_element)
        (if (Actor|ActorHasTag (Variables|Cam|GetCurrent%20Instance) "Forward")
          (Variables|Cam|SetForward%20Cam (Variables|Cam|GetCurrent%20Instance))
          (elif (Actor|ActorHasTag (Variables|Cam|GetCurrent%20Instance) "Left")
            (Variables|Cam|SetLeft%20Cam (Variables|Cam|GetCurrent%20Instance))
            (elif (Actor|ActorHasTag (Variables|Cam|GetCurrent%20Instance) "Right")
              (Variables|Cam|SetRight%20Cam (Variables|Cam|GetCurrent%20Instance))
              (elif (Actor|ActorHasTag (Variables|Cam|GetCurrent%20Instance) "StartCam")
                (Variables|Cam|SetStart%20Cam (Variables|Cam|GetCurrent%20Instance))
                (elif (Actor|ActorHasTag (Variables|Cam|GetCurrent%20Instance) "Bottem")
                  (Variables|Cam|SetBottem%20Cam (Variables|Cam|GetCurrent%20Instance)))))))))
    (:then_1
      (if (Variables|Default|GetStart%20Initial%20Seqeunce?)
        (Game|Player|SetViewTargetwithBlend (Game|GetPlayerController 0) (Variables|Cam|GetStart%20Cam) 1.0 "VTBlend_PreBlended" 0.0 true)
        (Utilities|FlowControl|Delay 2.0)
        (Game|Player|SetViewTargetwithBlend (Game|GetPlayerController 0) (Variables|Cam|GetForward%20Cam) 2.0 "VTBlend_Cubic" 0.0 true)
        (Utilities|FlowControl|Delay 2.0)
        (CallFunction|EndInitialCutScene)
        (else
          (CallFunction|EndInitialCutScene))))
    (:then_2
      (bind _returnvalue (UserInterface|CreateWidget "/Game/BP/Widget/Widget_Menu.Widget_Menu_C"))
      (bind _output_get (Variables|Default|SetMenu%20widget _returnvalue))
      (UserInterface|Viewport|AddtoViewport _output_get 0))))

(event Input|KeyboardEvents|W
  (params (Key :type Key%20Structure :default "None"))
  (bind _forward_cam (Variables|Cam|GetForward%20Cam))
  ;[1 1 1] Controls
  (:Pressed
    (Utilities|CamLocked?
      (:else
        (Game|Player|SetViewTargetwithBlend (Game|GetPlayerController 0) _forward_cam 1.0 "VTBlend_Cubic" 0.0 true)
        (Utilities|HideArms)
        (Utilities|ShowArms _forward_cam)))))

(event Input|KeyboardEvents|D
  (params (Key :type Key%20Structure :default "None"))
  (bind _right_cam (Variables|Cam|GetRight%20Cam))
  ;[1 1 1] Controls
  (:Pressed
    (Utilities|CamLocked?
      (:else
        (Game|Player|SetViewTargetwithBlend (Game|GetPlayerController 0) _right_cam 1.0 "VTBlend_Cubic" 0.0 true)
        (Utilities|HideArms)
        (Utilities|ShowArms _right_cam)))))

(event Input|KeyboardEvents|4
  (params (Key :type Key%20Structure :default "None"))
  (:Pressed
    (Variables|Default|SetPotion%20Type "NewEnumerator2")))

(event Input|KeyboardEvents|5
  (params (Key :type Key%20Structure :default "None"))
  (:Pressed
    (Variables|Default|SetPotion%20Type "NewEnumerator1")))

(event Input|KeyboardEvents|A
  (params (Key :type Key%20Structure :default "None"))
  (bind _left_cam (Variables|Cam|GetLeft%20Cam))
  ;[1 1 1] Controls
  (:Pressed
    (Utilities|CamLocked?
      (:else
        (Game|Player|SetViewTargetwithBlend (Game|GetPlayerController 0) _left_cam 1.0 "VTBlend_Cubic" 0.0 true)
        (Utilities|HideArms)
        (Utilities|ShowArms _left_cam)))))

(event Input|MouseEvents|LeftMouseButton
  (params (Key :type Key%20Structure :default "None"))
  (bind _returnvalue (Game|GetPlayerController 0))
  (bind _inventory (Variables|Default|GetInventory))
  (bind _hitresult (Game|Player|GetHitResultUnderCursorbyChannel _returnvalue "TraceTypeQuery1" true))
  ;[1 1 1] Pick Up
  (:Pressed
    (if (Utilities|DoesObjectImplementInterface (.hitactor _hitresult) "/Game/BP/BPI/BPI_ItemObjects.BPI_ItemObjects_C")
      (bind _asbp_item_object (Utilities|Casting|CastToBP_ItemObject (.hitactor _hitresult)))
      (Utilities|Array|Add (Variables|Default|GetCollectedItems) (Variables|/Game/BP/Item/BP_ItemObject.BP_ItemObject_C|GetRootType _asbp_item_object))
      (Class|BPIItemObjects|PickUpObject(Message) (.hitactor _hitresult))
      (Default|PlayHandAnimation (Variables|Cam|GetCurrentCam))
      (elif (Utilities|DoesObjectImplementInterface (.hitactor _hitresult) "/Game/BP/BPI/BPI_Cauldron.BPI_Cauldron_C")
        (Class|BPICauldron|Confirm(Message) (.hitactor _hitresult))
        (Class|BPICauldron|FlipBook(Message) (.hitactor _hitresult))
        (elif (Utilities|DoesObjectImplementInterface (.hitactor _hitresult) "/Game/BP/BPI/BPI_Bowl.BPI_Bowl_C")
          (Class|BPIBowl|BowlSelected(Message) (.hitactor _hitresult))
          (else
            ;[1 1 1] left Click
            ;;[1 1 1] Replace with Hand
            (if (> (.Value (Utilities|Map|Find (Variables|Default|GetInventory) (Variables|Default|GetPotion%20Type))) 0)
              (Game|SpawnActorfromClass "/Game/BP/Item/BP_Potion.BP_Potion_C" (Math|Transform|MakeTransform (Transformation|GetWorldLocation (Variables|/Script/Engine.Actor|GetRootComponent (Variables|Cam|GetCurrentCam))) (Math|Conversions|RotationFromXVector (.WorldDirection (Game|Player|ConvertMouseLocationToWorldSpace (Game|GetPlayerController 0)))) "1.000000,1.000000,1.000000") "AlwaysSpawn" 0 (Variables|Default|GetPotion%20Type) 0)
              (bind _result (Math|Integer|DecrementInt (.Value (Utilities|Map|Find _inventory (Variables|Default|GetPotion%20Type))))
                (:%20%20
                  (Utilities|Map|Add _inventory (Variables|Default|GetPotion%20Type) _result)
                  (Default|PlayHandAnimation (Variables|Cam|GetCurrentCam)))))))))))

(event Input|KeyboardEvents|S
  (params (Key :type Key%20Structure :default "None"))
  (bind _bottem_cam (Variables|Cam|GetBottem%20Cam))
  ;[1 1 1] Controls
  (:Pressed
    (Utilities|CamLocked?
      (:else
        (Game|Player|SetViewTargetwithBlend (Game|GetPlayerController 0) _bottem_cam 1.0 "VTBlend_Cubic" 0.0 true)
        (Utilities|HideArms)
        (Utilities|ShowArms _bottem_cam)))))

(event Input|KeyboardEvents|Tab
  (params (Key :type Key%20Structure :default "None"))
  ;[1 1 1] Tab
  (:Pressed
    (if (Variables|Default|GetTab%20in%20Use?)
      (Utilities|IsValid (Variables|Widget|GetTab%20Menu)
        (:Is%20Valid
          (Utilities|FlowControl|DoOnce false
            (:Completed
              (UserInterface|Animation|PlayAnimation (Variables|Widget|GetTab%20Menu) (Variables|/Game/BP/Widget/Widget_TabMenu.Widget_TabMenu_C|GetScrollDown (Variables|Widget|GetTab%20Menu)) 0.0 1 "Forward" 2.0 false)
              (Utilities|FlowControl|Delay 0.5)
              (Widget|RemovefromParent (Variables|Widget|GetTab%20Menu))
              (Variables|Default|SetTab%20in%20Use? false)
              (CallFunction|ResetDoOnceTab)))))
      (else
        (Variables|Default|SetTab%20in%20Use? true)
        (bind _returnvalue (UserInterface|CreateWidget "/Game/BP/Widget/Widget_TabMenu.Widget_TabMenu_C"))
        (bind _output_get (Variables|Widget|SetTab%20Menu _returnvalue))
        (UserInterface|Viewport|AddtoViewport _output_get 0)))))

(event Input|KeyboardEvents|1
  (params (Key :type Key%20Structure :default "None"))
  (:Pressed
    (Variables|Default|SetPotion%20Type "NewEnumerator0")))

(event Input|KeyboardEvents|2
  (params (Key :type Key%20Structure :default "None"))
  (:Pressed
    (Variables|Default|SetPotion%20Type "NewEnumerator4")))

(event Input|KeyboardEvents|3
  (params (Key :type Key%20Structure :default "None"))
  (:Pressed
    (Variables|Default|SetPotion%20Type "NewEnumerator3")))

(fn ConstructionScript)

(fn EndInitialCutScene
  (Variables|Cam|SetCam%20movement%20Locked false)
  (Variables|/Script/Engine.PlayerController|SetbShowMouseCursor (Game|GetPlayerController 0) true))

(fn SetFirstCamOveride
  (Game|Player|SetViewTargetwithBlend (Game|GetPlayerController 0) (Variables|Cam|GetForward%20Cam) 1.0 "VTBlend_Cubic" 0.0 true))