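; BP_CamSetting is a character-side Blueprint that controls the visibility and animation of a hands skeletal mesh, SKHands2.
; BeginPlay hides the hands and caches the Billboard component's relative location as the resting position.
; ShowHands snaps the Billboard back along X, waits briefly, unhides the mesh, then uses a timeline lerp to slide the Billboard to the cached position.
; PlayHandAnimation plays a supplied montage on the hands.
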(event Custom|ShowHands
  (Transformation|SetRelativeLocation (Variables|Default|GetBillboard) "-100.000000,0.000000,0.000000" false false)
  (Utilities|FlowControl|Delay 1.0)
  (Development|SetHiddeninGame (Variables|Default|GetSK_Hands_2) false false)
  (bind _newtrack_0 (Timeline|Timeline PlayFromStart)
    (:Update
      (Transformation|SetRelativeLocation (Variables|Default|GetBillboard) (Math|Vector|Lerp(Vector) "-100.000000,0.000000,0.000000" (Variables|Default|GetCurrent%20Location) _newtrack_0) false false))))

(event Custom|HideHands
  (Development|SetHiddeninGame (Variables|Default|GetSK_Hands_2) true false))

(event Custom|PlayHandAnimation
  (params (MontageToPlay :type Anim%20Montage%20Object%20Reference))
  (Animation|Montage|PlayMontage (Variables|Default|GetSK_Hands_2) MontageToPlay))

(event EventBeginPlay
  (CallFunction|HideHands)
  (Variables|Default|SetCurrent%20Location (Variables|/Script/Engine.SceneComponent|GetRelativeLocation (Variables|Default|GetBillboard))))

(fn ConstructionScript)