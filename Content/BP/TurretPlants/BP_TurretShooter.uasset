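; BP_TurretShooter is a plant turret that fires automatically along its fire point's forward direction on a looping, randomly timed timer.
; A montage notify triggers each shot, a sphere trace that sends a damage message and spends one Health, stopping at zero.
; Boost temporarily quickens firing and animation, while Upgrade temporarily widens the trace and doubles damage, both using retriggerable delays.
; Heal restores Health.
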(event Custom|Shoot
  (bind _firepoint (Variables|Default|GetFirePoint))
  (bind _returnvalue (Transformation|GetWorldLocation _firepoint))
  (Animation|Montage|PlayMontage (Variables|Default|GetSkeletalMesh) "/Game/Art/Animations/Plants/Plant_Anim_Montage.Plant_Anim_Montage" (Math|Float|SelectFloat 2.0 1.0 (Variables|Default|GetBoosted))
    (:OnNotifyBegin
      (if (not (<= (Variables|Default|GetHealth) 0.0))
        (bind _outhit (Collision|SphereTraceByChannel _returnvalue (+ _returnvalue (* (Math|Vector|GetForwardVector _firepoint) 1e+07)) (Math|Float|SelectFloat 1e+02 5e+01 (Variables|Default|GetUpgraded)) "TraceTypeQuery1" true 0 "None" true "(R=1.000000,G=0.000000,B=0.000000,A=1.000000)" "(R=0.000000,G=1.000000,B=0.000000,A=1.000000)" 1.0))
        (Math|Float|DecrementFloat (Variables|Default|GetHealth)
          (:%20%20
            (Class|BPIEnemy|DealDamage(Message) (.HitActor (Collision|BreakHitResult _outhit)) (Math|Float|SelectFloat 2e+01 1e+01 (Variables|Default|GetUpgraded)))
            (Components|Activation|Activate (Variables|Default|GetP_Shot_01) true)))))))

(event EventUpgrade
  (Development|PrintString "Upgraded")
  (Variables|Default|SetUpgraded true)
  (Animation|Montage|PlayMontage (Variables|Default|GetSkeletalMesh) "/Game/Art/Animations/Plants/plantHappy_Montage.plantHappy_Montage"
    (:then
      (Utilities|FlowControl|RetriggerableDelay 15.0)
      (Variables|Default|SetUpgraded false))))

(event EventHeal
  (Variables|Default|SetHealth 6e+01))

(event EventBoost
  (Animation|Montage|PlayMontage (Variables|Default|GetSkeletalMesh) "/Game/Art/Animations/Plants/plantHappy_Montage.plantHappy_Montage"
    (:then
      (bind _returnvalue (Utilities|Time|SetTimerbyEvent (delegate Custom|Shoot) 1.0 true))
      (Development|PrintString "Boosted")
      (Variables|Default|SetBoosted true)
      (Utilities|Time|PauseTimerbyHandle (Variables|Default|GetShootTimer))
      (Utilities|FlowControl|RetriggerableDelay 15.0)
      (Variables|Default|SetBoosted false)
      (Utilities|Time|PauseTimerbyHandle _returnvalue)
      (Utilities|Time|ClearandInvalidateTimerbyHandle _returnvalue)
      (Utilities|Time|SetTimerbyEvent (delegate Custom|Shoot) (Math|Random|RandomFloatinRange 3.0 5.0) true))))

(event EventBeginPlay
  (bind _returnvalue (Utilities|Time|SetTimerbyEvent (delegate Custom|Shoot) (Math|Random|RandomFloatinRange 3.0 5.0) true))
  (Variables|Default|SetShootTimer _returnvalue))

(fn ConstructionScript)