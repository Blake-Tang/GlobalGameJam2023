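; BP_Enem is an enemy that follows a spline path and flags itself as attacking near the end.
; A timeline, with play rate set by EnemySpeed, moves the skeletal mesh along the spline.
; DealDamage reduces health, while explosions kill outright; death spawns a hit effect and item before destroying the actor.
; BrambleSlow cuts speed to a fifth, but its delayed restore is unwired, so the slow persists.
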(event Custom|Death
  (bind _p_asteroid_hit (Variables|Default|GetP_Asteroid_Hit))
  (bind _returnvalue (Transformation|GetWorldLocation _p_asteroid_hit))
  (Niagara|SpawnSystematLocation "/Game/Stylized_VFX_StPack/Particles/UPDATE_1_3/P_Asteroid_Hit.P_Asteroid_Hit" _returnvalue)
  (Game|SpawnActorfromClass "/Game/BP/Item/BP_ItemObject.BP_ItemObject_C" (Math|Transform|MakeTransform _returnvalue "0, 0, 0" "2.000000,2.000000,2.000000") "Undefined" 0 "NewEnumerator0" 0)
  (Actor|DestroyActor))

(event EventBeginPlay
  (bind _asbp_base_character (Utilities|Casting|CastToBP_BaseCharacter (Game|Player|GetPlayerPawn 0)))
  (Variables|Default|SetAs%20BP%20Base%20Character _asbp_base_character)
  (Components|Timeline|SetPlayRate (Variables|Default|GetMoving%20Timeline) (Variables|Default|GetEnemy%20Speed))
  (Variables|Default|SetStored%20Speed (Variables|Default|GetEnemy%20Speed))
  (bind _alpha (Timeline|Moving%20Timeline PlayFromStart)
    (:Update
      (Variables|Default|SetAlpha_0 _alpha)
      (Transformation|SetWorldLocation (Variables|Default|GetSkeletalMesh) (Spline|GetLocationatDistanceAlongSpline (Variables|Default|GetSpline) (Math|Float|Lerp 0.0 (Spline|GetSplineLength (Variables|Default|GetSpline)) (Variables|Default|GetAlpha_0)) "World") false false)
      (if (>= (Variables|Default|GetAlpha_0) 0.99)
        (Variables|Default|SetAttacking? true)))))

(event EventExplosionDamage
  (CallFunction|Death))

(event EventBrambleSlow
  (Components|Activation|Activate (Variables|Default|GetP_StoneShield_01) true)
  (Components|Timeline|SetPlayRate (Variables|Default|GetMoving%20Timeline) (/ (Variables|Default|GetStored%20Speed) 5.0)))

(event EventDealDamage
  (params (DMG :type Float%20%28double-precision%29))
  (Variables|Default|SetHealth (- (Variables|Default|GetHealth) DMG))
  (Components|Activation|Activate (Variables|Default|GetP_Liquid_Hit_03) true)
  (if (<= (Variables|Default|GetHealth) 0.0)
    (CallFunction|Death)))

(fn ConstructionScript)