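; Enemy spawner that places BP_Enem actors at the first point of its spline, facing the PlayerStart location.
; BeginPlay caches that location and triggers SpawnMore, a self-repeating loop on a randomized, clamped Delay.
; Each spawn passes the spline and a rising speed to the enemy, and shortens later delays to ramp difficulty.
; Timer and spline-movement nodes are disconnected leftovers; AddPointIndex only increments an index and plays MoveTimeline.
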(event Custom|Add%20Point%20Index
  (Math|Integer|IncrementInt (Variables|Default|GetPoint%20Index)
    (:%20%20
      (Timeline|Move%20Timeline PlayFromStart))))

(event Custom|Spawn%20More
  (bind _spawn_time_max (Variables|Default|GetSpawn%20Time%20Max))
  (Utilities|FlowControl|Delay (Math|Float|Clamp(Float) (- (Math|Random|RandomFloatinRange 2e+01 _spawn_time_max) (Variables|Default|GetSpawn%20Time%20Deduction)) 2.0 _spawn_time_max) :!label _label)
  (Variables|Default|SetDifficulty%20Speed (+ (Variables|Default|GetDifficulty%20Speed) 0.01))
  (Game|SpawnActorfromClass "/Game/BP/Enemy/BP_Enem.BP_Enem_C" (Math|Transform|MakeTransform (Spline|GetLocationatSplinePoint (Variables|Default|GetSpline) 0 "World") (Math|Rotator|FindLookatRotation (Transformation|GetWorldLocation (Variables|Default|GetDefaultSceneRoot)) (Variables|Default|GetPlayerLocation)) "1.000000,1.000000,1.000000") "Undefined" 0 (Variables|Default|GetSpline) (+ (Variables|Default|GetEnemy%20Speed) (Variables|Default|GetDifficulty%20Speed)) 0)
  (Development|PrintString (Utilities|String|ToString(Float) (+ (Variables|Default|GetEnemy%20Speed) (Variables|Default|GetDifficulty%20Speed))))
  (Variables|Default|SetSpawn%20Time%20Deduction (+ (Variables|Default|GetSpawn%20Time%20Deduction) 0.5))
  (goto _label))

(event Collision|EventActorBeginOverlap
  (params (OtherActor :type Actor%20Object%20Reference)))

(event EventTick
  (params (DeltaSeconds :type Float%20%28single-precision%29)))

(event EventBeginPlay
  (bind _returnvalue (Actor|GetActorOfClass "/Script/Engine.PlayerStart"))
  (bind _output_get (Variables|Default|SetPlayerStart _returnvalue))
  (bind _output_get_2 (Variables|Default|SetPlayerLocation (Transformation|GetActorLocation _output_get)))
  (Development|PrintString (Utilities|String|ToString(Vector) _output_get_2))
  (Utilities|FlowControl|Sequence
    (:then_0
      ;[1 1 1] First Enemy
      (Utilities|FlowControl|Delay (Math|Random|RandomFloatinRange 2.0 2e+01))
      (CallFunction|SpawnMore))
    (:then_1
      (CallFunction|SpawnMore))))

(fn ConstructionScript)